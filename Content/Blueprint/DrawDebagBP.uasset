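; DrawDebagBP is a debug helper that draws colour-coded forward, right and up arrows for an actor's rotation.
; Its DrawDebagMarker event feeds actor rotation and distance from world origin into DrawDebag, which can also print the forward vector.
; Arrows lie on axes through the world origin, pointing inward to roughly that distance, rather than starting at the actor.
; BeginPlay caches the RMouseControler, and an unconnected nested loop over socket directions never runs.
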(event Custom|DrawDebagMarker
  (params (Show? :type Boolean) (ShowALL :type Boolean) (bPrintToScreen :type Boolean) (Location :type Actor%20Object%20Reference) (Rotation :type Actor%20Object%20Reference))
  (bind _returnvalue (Transformation|GetActorLocation Location))
  (bind _returnvalue_2 (Math|Vector|VectorLength _returnvalue))
  (CallFunction|DrawDebag Show? ShowALL ShowALL ShowALL 1e+02 5e+01 1e+01 (Transformation|GetActorRotation Rotation) _returnvalue_2 (+ _returnvalue_2 2e+02) bPrintToScreen))

(event EventBeginPlay
  (bind _asrmouse_controler (Utilities|Casting|CastToRMouseControler (Game|GetPlayerController 0)))
  (Variables|Default|SetControlerReference _asrmouse_controler))

(fn ConstructionScript)

(fn DrawDebag
  (params (Condition :type Boolean) (Condition1 :type Boolean) (Condition2 :type Boolean) (Condition3 :type Boolean) (ArrowSize :type Float%20%28single-precision%29) (Duration :type Float%20%28single-precision%29) (Thickness :type Float%20%28single-precision%29) (InRot :type Rotator) (B :type Float%20%28single-precision%29) (A :type Float%20%28single-precision%29) (bPrintToScreen :type Boolean))
  (bind _returnvalue (Math|Vector|GetForwardVector InRot))
  (bind _returnvalue_2 (Math|Vector|GetRightVector InRot))
  (bind _returnvalue_3 (Math|Vector|GetUpVector InRot))
  (if Condition
    (if Condition1
      (Development|PrintString (Utilities|String|ToString(Vector) _returnvalue) bPrintToScreen true "(R=0.000000,G=0.660000,B=1.000000,A=1.000000)" Duration)
      (Rendering|Debug|DrawDebugArrow (* _returnvalue A) (+ _returnvalue (* _returnvalue B)) ArrowSize "(R=0.540000,G=0.046757,B=0.003734,A=1.000000)" Duration Thickness))
    (if Condition2
      (Rendering|Debug|DrawDebugArrow (* _returnvalue_2 A) (+ _returnvalue_2 (* _returnvalue_2 B)) ArrowSize "(R=0.012667,G=0.440000,B=0.072977,A=1.000000)" Duration Thickness))
    (if Condition3
      (Rendering|Debug|DrawDebugArrow (* _returnvalue_3 A) (+ _returnvalue_3 (* _returnvalue_3 B)) ArrowSize "(R=0.000000,G=0.042804,B=0.530000,A=1.000000)" Duration Thickness)
      (return)
      (else
        _)))
  (return))