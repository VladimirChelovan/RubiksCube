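; RPlayer is the player camera actor for a Rubik's Cube game, with a spring arm centered on the cube and mouse wheel zoom.
; BeginPlay finds the first RubiksCube, teleports to it, and caches references to it and the RMouseControler.
; Mouse wheel input changes spring arm length within clamped limits, stepping out faster than in.
; Tick sets the actor to the spring arm's own location through a zero-speed VInterpTo, so no smoothing occurs.
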(event EventBeginPlay
  ;[1 1 1] Cast, set location orbit
  (bind _outactors (Actor|GetAllActorsOfClass "/Game/Blueprint/RubiksCube.RubiksCube_C"))
  (bind _asrubiks_cube (Utilities|Casting|CastToRubiksCube (Utilities|Array|Get(acopy) _outactors)))
  (bind _output_get (Variables|Default|SetRubiksReference _asrubiks_cube))
  (Transformation|SetActorLocation (Transformation|GetActorLocation _output_get) true true)
  (bind _asrmouse_controler (Utilities|Casting|CastToRMouseControler (Game|GetPlayerController 0)))
  (Variables|Default|SetControlerReference _asrmouse_controler))

(event EventTick
  (params (DeltaSeconds :type Float%20%28single-precision%29))
  (bind _springarm (Variables|Default|GetSpringArm))
  ;[1 1 1] Cube Orbit
  (Transformation|SetActorLocation (Math|Interpolation|VInterpTo (Transformation|GetWorldLocation _springarm) (Transformation|GetWorldLocation _springarm) 0.0 0.0) false false))

(event Input|MouseEvents|MouseWheelDown
  (params (Key :type Key%20Structure :default "AnyKey"))
  (bind _springarm (Variables|Default|GetSpringArm))
  ;[1 1 1] Zoom
  (:Pressed
    (Variables|/Script/Engine.SpringArmComponent|SetTargetArmLength _springarm (Math|Float|Clamp(Float) (+ (Variables|/Script/Engine.SpringArmComponent|GetTargetArmLength _springarm) 2.5e+02) 1e+03 2e+03))))

(event Input|MouseEvents|MouseWheelUp
  (params (Key :type Key%20Structure :default "AnyKey"))
  (bind _springarm (Variables|Default|GetSpringArm))
  ;[1 1 1] Zoom
  (:Pressed
    (Variables|/Script/Engine.SpringArmComponent|SetTargetArmLength _springarm (Math|Float|Clamp(Float) (- (Variables|/Script/Engine.SpringArmComponent|GetTargetArmLength _springarm) 1e+02) 1e+03 2e+03))))

(fn ConstructionScript)