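; Mouse controller for a Rubik's Cube game that rotates the view on empty-space drags, picks layers on cube drags and creates the UI widget.
; Dragging between two pieces sets a direction sign from mouse movement, while line traces derive four anchor pieces.
; Box traces between anchors collect the layer, and a nine-piece selection triggers CheckMaxZXY on the cube.
; StartRotation feeds randomly chosen cube axis arrays into that selection for scrambling.
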(event Custom|Reset
  ;[1 1 1] Next Component Select
  (Utilities|FlowControl|DoOnce true) ; enters at Reset
)

(event Custom|ResetDirection
  (bind _returnvalue (Game|GetPlayerController 0))
  (bind (_locationx _locationy) (Class|WidgetLayoutLibrary|GetMousePositionScaledbyDPI _returnvalue))
  ;[1 1 1] Direction from the position
  (Utilities|FlowControl|Sequence
    (:then_0
      (Utilities|FlowControl|DoOnce true) ; enters at Reset
    )
    (:then_1
      (Utilities|FlowControl|DoOnce true) ; enters at Reset
    )))

(event Custom|Select%20Array%20and%20Cast%20to%20Cube
  (bind _drawdebagtype (Variables|DrawDebag|GetDrawDebagType))
  (bind _objecttype (Variables|DrawDebag|GetObjecttype))
  (bind _vector_array (Variables|SelectComponent|GetVector%20array))
  (bind _item (Utilities|Array|Get(acopy) _vector_array))
  (bind _item_2 (Utilities|Array|Get(acopy) _vector_array 1))
  (bind _item_3 (Utilities|Array|Get(acopy) _vector_array 2))
  (bind _item_4 (Utilities|Array|Get(acopy) _vector_array 3))
  ;[1 1 1] Create array and cast to cube
  (Utilities|Array|Clear (Variables|SelectComponent|GetSelect%20Array))
  (Utilities|FlowControl|Sequence
    (:then_0
      (bind _outhits (Class|KismetSystemLibrary|BoxTraceMultiforObjects _item _item_2 "90.000000,90.000000,90.000000" "0, 0, 0" _objecttype false 0 _drawdebagtype false))
      (CallFunction|DebagMultyLineTrace(addArray) _outhits true))
    (:then_1
      (bind _outhits_2 (Class|KismetSystemLibrary|BoxTraceMultiforObjects _item_3 _item_2 "90.000000,90.000000,90.000000" "0, 0, 0" _objecttype false 0 _drawdebagtype false))
      (CallFunction|DebagMultyLineTrace(addArray) _outhits_2 true))
    (:then_2
      (bind _outhits_3 (Class|KismetSystemLibrary|BoxTraceMultiforObjects _item_2 _item_4 "90.000000,90.000000,90.000000" "0, 0, 0" _objecttype false 0 _drawdebagtype false))
      (CallFunction|DebagMultyLineTrace(addArray) _outhits_3 true))
    (:then_3
      (bind _outhits_4 (Class|KismetSystemLibrary|BoxTraceMultiforObjects _item _item_4 "90.000000,90.000000,90.000000" "0, 0, 0" _objecttype false 0 _drawdebagtype false))
      (CallFunction|DebagMultyLineTrace(addArray) _outhits_4 true))
    (:then_4
      (bind _outhits_5 (Class|KismetSystemLibrary|BoxTraceMultiforObjects _item_2 _item "90.000000,90.000000,90.000000" "0, 0, 0" _objecttype false 0 _drawdebagtype false))
      (CallFunction|DebagMultyLineTrace(addArray) _outhits_5 true))
    (:then_5
      (bind _outhits_6 (Class|KismetSystemLibrary|BoxTraceMultiforObjects _item_3 _item_4 "90.000000,90.000000,90.000000" "0, 0, 0" _objecttype false 0 _drawdebagtype false))
      (CallFunction|DebagMultyLineTrace(addArray) _outhits_6 true)
      ;[1 1 1] Fix
      (bind _9_ (CallFunction|SmalFix false))
      (if _9_
        (Variables|SelectComponent|SetSelectComponentCubeOne 0)
        (Variables|SelectComponent|SetSelectComponentCubeOne 0)
        (Variables|SelectComponent|SetSelectComponentCubeThree 0)
        (Variables|SelectComponent|SetSelectComponentCubeFour 0)
        (Default|CheckMaxZXY (Variables|Cast|GetCubeReference))
        (else
          (Variables|SelectComponent|SetSelectComponentCubeOne 0)
          (Variables|SelectComponent|SetSelectComponentCubeOne 0)
          (Variables|SelectComponent|SetSelectComponentCubeThree 0)
          (Variables|SelectComponent|SetSelectComponentCubeFour 0))))))

(event Custom|Direction1
  (bind _returnvalue (Game|GetPlayerController 0))
  (bind (_locationx _locationy) (Class|WidgetLayoutLibrary|GetMousePositionScaledbyDPI _returnvalue))
  ;[1 1 1] Direction from the position
  (Utilities|FlowControl|DoOnce true
    (:Completed
      (bind _output_get (Variables|DirectionAnimation|SetFirstXposition _locationx))
      (bind _output_get_2 (Variables|DirectionAnimation|SetFirstYposition _locationy)))))

(event Custom|Direction2
  (bind _returnvalue (Game|GetPlayerController 0))
  (bind (_locationx _locationy) (Class|WidgetLayoutLibrary|GetMousePositionScaledbyDPI _returnvalue))
  ;[1 1 1] Direction from the position
  (Utilities|FlowControl|DoOnce true
    (:Completed
      (bind _output_get (Variables|DirectionAnimation|SetTwoXposition _locationx))
      (bind _output_get_2 (Variables|DirectionAnimation|SetTwoYposition _locationy))
      (if (> (Math|Float|Absolute(Float) (- (stale Custom|Direction1 _output_get) _output_get)) (Math|Float|Absolute(Float) (- (stale Custom|Direction1 _output_get_2) _output_get_2)))
        (if (> (stale Custom|Direction1 _output_get) _output_get)
          (Variables|DirectionAnimation|SetDirectionAnimation 1.0)
          (else
            (Variables|DirectionAnimation|SetDirectionAnimation -1.0)))
        (elif (> (stale Custom|Direction1 _output_get_2) _output_get_2)
          (Variables|DirectionAnimation|SetDirectionAnimation -1.0)
          (else
            (Variables|DirectionAnimation|SetDirectionAnimation 1.0)))))))

(event Custom|Select%20all
  (bind _selectcomponentcubeone (Variables|SelectComponent|GetSelectComponentCubeOne))
  (bind _objecttype (Variables|DrawDebag|GetObjecttype))
  (bind _returnvalue (Transformation|GetActorLocation _selectcomponentcubeone))
  ;[1 1 1] Create grids capture, to select components.
  (bind _outhit (Collision|LineTraceByChannel (.WorldLocation (Game|Player|ConvertMouseLocationToWorldSpace (Game|GetPlayerController 0))) (Transformation|GetActorLocation (Variables|SelectComponent|GetSelectComponentCubeOne)) "TraceTypeQuery1" false 0 "None" false))
  (bind _outhits (Class|KismetSystemLibrary|LineTraceMultiforObjects (.Location (Collision|BreakHitResult _outhit)) (- (.Location (Collision|BreakHitResult _outhit)) (* (.ImpactNormal (Collision|BreakHitResult _outhit)) 1.2e+03)) (Variables|DrawDebag|GetObjecttype) false 0 "None" true))
  (if (Components|ComponentHasTag (Class|Actor|GetParentComponent (.HitActor (Collision|BreakHitResult (Utilities|Array|Get(acopy) _outhits 2)))) "Cube")
    (Variables|SelectComponent|SetSelectComponentCubeFour (.HitActor (Collision|BreakHitResult (Utilities|Array|Get(acopy) _outhits 2))))
    (bind _outhits_2 (Class|KismetSystemLibrary|LineTraceMultiforObjects (Transformation|GetActorLocation (.HitActor (Collision|BreakHitResult (Utilities|Array|Get(acopy) (stale Custom|Select%203%20and _outhits) (Utilities|Array|LastIndex (stale Custom|Select%203%20and _outhits)))))) (+ (Transformation|GetActorLocation (.HitActor (Collision|BreakHitResult (Utilities|Array|Get(acopy) (stale Custom|Select%203%20and _outhits) (Utilities|Array|LastIndex (stale Custom|Select%203%20and _outhits)))))) (* (* (Math|Vector|GetForwardVector (Math|Rotator|FindLookatRotation (Transformation|GetActorLocation (.HitActor (Collision|BreakHitResult (Utilities|Array|Get(acopy) _outhits 2)))) (Transformation|GetActorLocation (.HitActor (Collision|BreakHitResult (Utilities|Array|Get(acopy) (stale Custom|Select%203%20and _outhits) (Utilities|Array|LastIndex (stale Custom|Select%203%20and _outhits)))))))) 2.7e+02) -1.0)) _objecttype false 0 "None" true "(R=0.532752,G=0.165041,B=1.000000,A=1.000000)" "(R=1.000000,G=0.071664,B=0.000000,A=1.000000)"))
    (bind _outhits_3 (Class|KismetSystemLibrary|LineTraceMultiforObjects _returnvalue (+ _returnvalue (* (Math|Vector|GetForwardVector (Math|Rotator|FindLookatRotation _returnvalue (.TraceEnd (Collision|BreakHitResult (Utilities|Array|Get(acopy) _outhits_2 (Utilities|Array|LastIndex _outhits_2)))))) 1.2e+03)) _objecttype false 0 "None" true "(R=0.082387,G=0.960197,B=1.000000,A=1.000000)" "(R=0.000000,G=0.266184,B=1.000000,A=1.000000)"))
    (if (Components|ComponentHasTag (Class|Actor|GetParentComponent (.HitActor (Collision|BreakHitResult (Utilities|Array|Get(acopy) _outhits_3 (Utilities|Array|LastIndex _outhits_3))))) "Cube")
      (Variables|SelectComponent|SetSelectComponentCubeTwo (.HitActor (Collision|BreakHitResult (Utilities|Array|Get(acopy) _outhits_3 (Utilities|Array|LastIndex _outhits_3)))))
      (CallFunction|CreateVectorArray))))

(event Custom|Select%203%20and
  (bind _selectcomponentcubeone (Variables|SelectComponent|GetSelectComponentCubeOne))
  (bind _selectcomponentcubetwo (Variables|SelectComponent|GetSelectComponentCubeTwo))
  (bind _returnvalue (Transformation|GetActorLocation _selectcomponentcubetwo))
  (bind _returnvalue_2 (Transformation|GetActorLocation _selectcomponentcubeone))
  (bind _returnvalue_3 (Math|Rotator|FindLookatRotation _returnvalue_2 _returnvalue))
  (bind _returnvalue_4 (Math|Vector|GetForwardVector _returnvalue_3))
  ;[1 1 1] Create grids capture, to select components.
  (bind _outhits (Class|KismetSystemLibrary|LineTraceMultiforObjects (+ (* (* _returnvalue_4 4e+02) -1.0) _returnvalue_2) (+ _returnvalue_2 (* _returnvalue_4 1.2e+03)) (Variables|DrawDebag|GetObjecttype) false 0 "None" true))
  (if (Components|ComponentHasTag (Class|Actor|GetParentComponent (.HitActor (Collision|BreakHitResult (Utilities|Array|Get(acopy) _outhits (Utilities|Array|LastIndex _outhits))))) "Cube")
    (Variables|SelectComponent|SetSelectComponentCubeThree (.HitActor (Collision|BreakHitResult (Utilities|Array|Get(acopy) _outhits (Utilities|Array|LastIndex _outhits)))))))

(event Custom|StartRotation
  (bind _cubereference (Variables|Cast|GetCubeReference))
  ;[1 1 1] RandomRotation
  (if (not (== (Variables|Default|GetRotationStart) 0))
    (Variables|Default|SetRotationStart (- (Variables|Default|GetRotationStart) 1))
    (switch int (Math|Random|RandomIntegerinRange 0 8)
      (:0
        (CallFunction|RandomStartRotation (Variables|/Game/Blueprint/RubiksCube.RubiksCube_C|GetX+ _cubereference)))
      (:1
        (CallFunction|RandomStartRotation (Variables|/Game/Blueprint/RubiksCube.RubiksCube_C|GetX0 _cubereference)))
      (:2
        (CallFunction|RandomStartRotation (Variables|/Game/Blueprint/RubiksCube.RubiksCube_C|GetX- _cubereference)))
      (:3
        (CallFunction|RandomStartRotation (Variables|/Game/Blueprint/RubiksCube.RubiksCube_C|GetZ+ _cubereference)))
      (:4
        (CallFunction|RandomStartRotation (Variables|/Game/Blueprint/RubiksCube.RubiksCube_C|GetZ0 _cubereference)))
      (:5
        (CallFunction|RandomStartRotation (Variables|/Game/Blueprint/RubiksCube.RubiksCube_C|GetZ- _cubereference)))
      (:6
        (CallFunction|RandomStartRotation (Variables|/Game/Blueprint/RubiksCube.RubiksCube_C|GetY+ _cubereference)))
      (:7
        (CallFunction|RandomStartRotation (Variables|/Game/Blueprint/RubiksCube.RubiksCube_C|GetY0 _cubereference)))
      (:8
        (CallFunction|RandomStartRotation (Variables|/Game/Blueprint/RubiksCube.RubiksCube_C|GetY- _cubereference))))))

(event Custom|Create%20Vector%20Array
  ;[1 1 1] Get location to vector array
  (Utilities|Array|Clear (Variables|SelectComponent|GetVector%20array))
  (Variables|SelectComponent|SetVector%20array (Utilities|Array|MakeArray (Transformation|GetActorLocation (Variables|SelectComponent|GetSelectComponentCubeOne)) (Transformation|GetActorLocation (Variables|SelectComponent|GetSelectComponentCubeTwo)) (Transformation|GetActorLocation (Variables|SelectComponent|GetSelectComponentCubeThree)) (Transformation|GetActorLocation (Variables|SelectComponent|GetSelectComponentCubeFour))))
  (Variables|Default|SetCountSelect (+ (Variables|Default|GetCountSelect) 1))
  (CallFunction|SelectArrayandCasttoCube))

(event EventTick
  (params (DeltaSeconds :type Float%20%28single-precision%29))
  (bind _objecttype (Variables|DrawDebag|GetObjecttype))
  (bind _hitresult (Class|PlayerController|GetHitResultUnderCursorforObjects _objecttype true))
  (bind _hitactor (Collision|BreakHitResult _hitresult))
  (bind _returnvalue (Class|Actor|GetParentComponent _hitactor))
  ;[1 1 1] Next Component Select
  (Utilities|FlowControl|Sequence
    (:then_0
      (if (and (Variables|Default|GetMousePress) (Variables|SelectComponent|GetCubeSelect))
        (if (Components|ComponentHasTag _returnvalue "Cube")
          (if (Utilities|Name|NotEqual(Name) (Utilities|Array|Get(acopy) (Variables|/Script/Engine.ActorComponent|GetComponentTags (Class|Actor|GetParentComponent (Variables|SelectComponent|GetSelectComponentCubeOne))) 1) (Utilities|Array|Get(acopy) (Variables|/Script/Engine.ActorComponent|GetComponentTags _returnvalue) 1))
            (Utilities|FlowControl|DoOnce true
              (:Completed
                (bind _output_get (Variables|SelectComponent|SetSelectComponentCubeTwo _hitactor))
                (CallFunction|Direction2)
                (if (!= (Variables|SelectComponent|GetSelectComponentCubeOne) _output_get)
                  (CallFunction|Select3and)
                  (CallFunction|SelectAll))))))))))

(event EventBeginPlay
  ;[1 1 1] Cast to Cube
  (bind _outactors (Actor|GetAllActorsOfClass "/Game/Blueprint/RubiksCube.RubiksCube_C"))
  (bind _asrubiks_cube (Utilities|Casting|CastToRubiksCube (Utilities|Array|Get(acopy) _outactors))
    (:then
      (Variables|Cast|SetCubeReference _asrubiks_cube)
      (CallFunction|ResetDirection)
      (bind _returnvalue (UserInterface|CreateWidget "/Game/Blueprint/Rwiget.Rwiget_C" (Game|GetPlayerController 0)))
      (UserInterface|Viewport|AddtoViewport _returnvalue 0))
    (:CastFailed
      (Development|PrintString "Error Cast cube"))))

(event Input|ActionEvents|InputActionLeftButtonMouse
  (params (Key :type Key%20Structure :default "AnyKey"))
  (bind _self self)
  (bind _objecttype (Variables|DrawDebag|GetObjecttype))
  (bind _hitresult (Class|PlayerController|GetHitResultUnderCursorforObjects _objecttype true))
  (bind _hitactor (Collision|BreakHitResult _hitresult))
  ;[1 1 1] Clicked mouse buton
  (:Pressed
    (if (not (Variables|/Game/Blueprint/RubiksCube.RubiksCube_C|GetPlayed (Variables|Cast|GetCubeReference)))
      (Variables|Default|SetMousePress true)
      (Variables|/Script/Engine.PlayerController|SetbShowMouseCursor _self false)
      (if (.ReturnValue (Game|Player|GetHitResultUnderCursorbyChannel "TraceTypeQuery2" true))
        (if (Components|ComponentHasTag (Class|Actor|GetParentComponent _hitactor) "Cube")
          (Variables|SelectComponent|SetCubeSelect true)
          (Variables|/Script/Engine.PlayerController|SetbShowMouseCursor self true)
          (Variables|SelectComponent|SetSelectComponentCubeOne _hitactor)
          (CallFunction|Direction1)))))
  (:Released
    (Variables|Default|SetMousePress false)
    (Variables|/Script/Engine.PlayerController|SetbShowMouseCursor _self true)
    (Variables|SelectComponent|SetCubeSelect false)
    (CallFunction|Reset)))

(event Input|AxisEvents|InputAxisLookLeft
  (params (AxisValue :type Float%20%28single-precision%29))
  ;[1 1 1] Camera Rotation Controls
  (if (Variables|Default|GetMousePress)
    (if (not (Variables|SelectComponent|GetCubeSelect))
      (Class|PlayerController|AddYawInput AxisValue))))

(event Input|AxisEvents|InputAxisLookUp
  (params (AxisValue :type Float%20%28single-precision%29))
  ;[1 1 1] Camera Rotation Controls
  (if (Variables|Default|GetMousePress)
    (if (not (Variables|SelectComponent|GetCubeSelect))
      (Class|PlayerController|AddPitchInput AxisValue))))

(fn ConstructionScript
  (|CallParentFunction))

(fn DebagMultyLineTrace(addArray)
  (params (InputPin :type Array%20of%20Hit%20Result%20Structures) (Show? :type Boolean))
  (if Show?
    (for _array_element InputPin
      (if (Components|ComponentHasTag (Class|Actor|GetParentComponent (.HitActor (Collision|BreakHitResult _array_element))) "Cube")
        (Rendering|Debug|DrawDebugBox (.TraceEnd (Collision|BreakHitResult _array_element)) "100.000000,100.000000,100.000000" "(R=0.146208,G=0.585000,B=0.579181,A=1.000000)" "0, 0,0.000000" 1.0 1e+01)
        (Utilities|Array|AddUnique (Variables|SelectComponent|GetSelect%20Array) (.HitActor (Collision|BreakHitResult _array_element)))))
    (return)
    (else
      (for _array_element_2 InputPin
        (if (Components|ComponentHasTag (Class|Actor|GetParentComponent (.HitActor (Collision|BreakHitResult _array_element_2))) "Cube")
          (Utilities|Array|AddUnique (Variables|SelectComponent|GetSelect%20Array) (.HitActor (Collision|BreakHitResult _array_element_2)))))
      (return))))

(fn SmalFix
  (params (Show? :type Boolean))
  (bind _select_array (Variables|SelectComponent|GetSelect%20Array))
  (bind _select_array_2 (Variables|SelectComponent|GetSelect%20Array))
  (bind _returnvalue (Utilities|Array|LastIndex _select_array_2))
  (bind _returnvalue_2 (Utilities|Array|LastIndex _select_array))
  (bind _returnvalue_3 (== _returnvalue 8))
  (bind _returnvalue_4 (== _returnvalue_2 8))
  (if Show?
    (if _returnvalue_4
      (return _returnvalue_4)
      (else
        (Development|PrintString "Error! Select Component" true true "(R=1.000000,G=0.380561,B=0.000000,A=1.000000)")
        (for _array_element _select_array
          (Development|PrintString (Utilities|GetDisplayName _array_element) true true "(R=1.000000,G=0.380561,B=0.000000,A=1.000000)" 1e+02)
          (return _returnvalue_4))))
    (elif _returnvalue_3
      (return _returnvalue_3)
      (else
        (return _returnvalue_3)))))

(fn RandomStartRotation
  (params (RandomSelect :type Array%20of%20Vectors))
  (Utilities|Array|Clear (Variables|SelectComponent|GetVector%20array))
  (for _array_element RandomSelect
    (Utilities|Array|Add (Variables|SelectComponent|GetVector%20array) _array_element))
  (if (Variables|Default|GetStartRotation?)
    (CallFunction|SelectArrayandCasttoCube))
  (return))